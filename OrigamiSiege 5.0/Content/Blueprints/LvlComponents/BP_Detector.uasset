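; BP_Detector is a lane detector that tracks the enemies and defenses in one line of a defense game.
; Overlapping actors tagged Enemy are cast by type tag, given a reference to the detector and added to EnemiesDetected.
; Each new enemy triggers UpdateDefenses on the GameManager so defenses in that line can attack.
; AddDefense registers archer, guard or fire defenses in DefendersLine and passes them the enemy list and detector reference.
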(event EventBeginPlay
  ;[1 1 1] Fill game manager variable
  (bind _returnvalue (Actor|GetActorOfClass "/Game/Blueprints/GameManager.GameManager_C"))
  (Variables|Default|SetGameManRef _returnvalue))

(event Collision|EventActorEndOverlap
  (params (OtherActor :type Actor%20Object%20Reference)))

(event EventTick
  (params (DeltaSeconds :type Float%20%28single-precision%29)))

(event Collision|EventActorBeginOverlap
  (params (OtherActor :type Actor%20Object%20Reference))
  (bind _self self)
  (bind _enemiesdetected (Variables|Default|GetEnemiesDetected))
  ;[1 1 1] Add new enemies on a list and update defenses to attack if they are in the same line
  (if (Actor|ActorHasTag OtherActor "Enemy")
    (bind _array_element (Utilities|Array|ForEachLoopwithBreak (Variables|/Script/Engine.Actor|GetTags OtherActor) :!label _label)
      (:LoopBody
        (switch name _array_element
          (:Basic
            (bind _asbp_basic_water (Utilities|Casting|CastToBP_BasicWater OtherActor))
            (Variables|/Game/Blueprints/Enemies/BP_BasicWater.BP_BasicWater_C|SetDetectorRef _asbp_basic_water _self)
            (Utilities|Array|Add _enemiesdetected _asbp_basic_water))
          (:Candle
            (bind _asbp_candle (Utilities|Casting|CastToBP_Candle OtherActor))
            (Variables|/Game/Blueprints/Enemies/BP_Candle.BP_Candle_C|SetDetectorRef _asbp_candle _self)
            (Utilities|Array|Add _enemiesdetected _asbp_candle))
          (:Wheel
            (bind _asbp_speed (Utilities|Casting|CastToBP_Speed OtherActor))
            (Variables|/Game/Blueprints/Enemies/BP_Speed.BP_Speed_C|SetDetectorRef _asbp_speed _self)
            (Utilities|Array|Add _enemiesdetected _asbp_speed))
          (:Throw
            (bind _asbp_thrower (Utilities|Casting|CastToBP_Thrower OtherActor))
            (Variables|/Game/Blueprints/Enemies/BP_Thrower.BP_Thrower_C|SetDetectorRef _asbp_thrower _self)
            (Utilities|Array|Add _enemiesdetected _asbp_thrower)))
        (Default|UpdateDefenses (Variables|Default|GetGameManRef) self)
        (goto _label Break)))))

(fn ConstructionScript)

(fn AddDefense
  (params (DefenseToAdd :type Actor%20Object%20Reference) (SelectedDefense :type Integer))
  (bind _self self)
  (bind _enemiesdetected (Variables|Default|GetEnemiesDetected))
  (Utilities|Array|Add (Variables|Default|GetDefendersLine) DefenseToAdd)
  (switch int SelectedDefense
    (:0
      (bind _asbp_archers (Utilities|Casting|CastToBP_Archers DefenseToAdd))
      (Variables|/Game/Blueprints/Defenses/BP_Archers.BP_Archers_C|SetEnemyList _asbp_archers _enemiesdetected)
      (Variables|/Game/Blueprints/Defenses/BP_Archers.BP_Archers_C|SetDetectorRef _asbp_archers _self))
    (:1
      (bind _asbp_guard (Utilities|Casting|CastToBP_Guard DefenseToAdd))
      (Variables|/Game/Blueprints/Defenses/BP_Guard.BP_Guard_C|SetEnemyList _asbp_guard _enemiesdetected)
      (Variables|/Game/Blueprints/Defenses/BP_Guard.BP_Guard_C|SetDetectorRef _asbp_guard _self))
    (:2
      (bind _asbp_fire (Utilities|Casting|CastToBP_Fire DefenseToAdd))
      (Variables|/Game/Blueprints/Defenses/BP_Fire.BP_Fire_C|SetEnemyList _asbp_fire _enemiesdetected)
      (Variables|/Game/Blueprints/Defenses/BP_Fire.BP_Fire_C|SetDetectorRef _asbp_fire _self)))
  (return))