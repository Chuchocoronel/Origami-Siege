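; BP_Spawner is a level actor that spawns enemies at its own transform, facing along its Arrow component's forward vector.
; SpawnEnemy looks up the given name in the TypeEnemiesData table, switches between BP_BasicWater and BP_Candle, and copies the row's health, speed, damage and attack timer onto the new enemy.
; A separate EnemySpawn event does the same, hardcoded to the Basic row.
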(event Custom|EnemySpawn
  (bind _returnvalue (Utilities|GetDataTableRow "/Game/Blueprints/Enemies/TypeEnemiesData.TypeEnemiesData" "Basic")
    (:then
      (bind _returnvalue_2 (Game|SpawnActorfromClass "/Game/Blueprints/Enemies/BP_BasicWater.BP_BasicWater_C" (Transformation|GetActorTransform) "Undefined" 0 0))
      (Variables|/Game/Blueprints/Enemies/BP_BasicWater.BP_BasicWater_C|SetDirection _returnvalue_2 (Math|Vector|GetForwardVector (Variables|Default|GetArrow)))
      (Variables|/Game/Blueprints/Enemies/BP_BasicWater.BP_BasicWater_C|SetHealth _returnvalue_2 (.health _returnvalue))
      (Variables|/Game/Blueprints/Enemies/BP_BasicWater.BP_BasicWater_C|SetSpeed _returnvalue_2 (.speed _returnvalue))
      (Variables|/Game/Blueprints/Enemies/BP_BasicWater.BP_BasicWater_C|SetEnemyDamage _returnvalue_2 (.damage _returnvalue))
      (Variables|/Game/Blueprints/Enemies/BP_BasicWater.BP_BasicWater_C|SetAttackTimer _returnvalue_2 (.attacktimer _returnvalue)))))

(event EventBeginPlay)

(event Collision|EventActorBeginOverlap
  (params (OtherActor :type Actor%20Object%20Reference)))

(event EventTick
  (params (DeltaSeconds :type Float%20%28single-precision%29)))

(fn ConstructionScript)

(fn SpawnEnemy
  (params (Enemy%20Name :type Name))
  (bind _returnvalue (Transformation|GetActorTransform))
  (bind _returnvalue_2 (Utilities|GetDataTableRow "/Game/Blueprints/Enemies/TypeEnemiesData.TypeEnemiesData" Enemy%20Name)
    (:then
      (switch name Enemy%20Name
        (:Basic
          (bind _returnvalue_3 (Game|SpawnActorfromClass "/Game/Blueprints/Enemies/BP_BasicWater.BP_BasicWater_C" _returnvalue "Undefined" 0 0))
          (Variables|/Game/Blueprints/Enemies/BP_BasicWater.BP_BasicWater_C|SetDirection _returnvalue_3 (Math|Vector|GetForwardVector (Variables|Default|GetArrow)))
          (Variables|/Game/Blueprints/Enemies/BP_BasicWater.BP_BasicWater_C|SetHealth _returnvalue_3 (.health _returnvalue_2))
          (Variables|/Game/Blueprints/Enemies/BP_BasicWater.BP_BasicWater_C|SetSpeed _returnvalue_3 (.speed _returnvalue_2))
          (Variables|/Game/Blueprints/Enemies/BP_BasicWater.BP_BasicWater_C|SetEnemyDamage _returnvalue_3 (.damage _returnvalue_2))
          (Variables|/Game/Blueprints/Enemies/BP_BasicWater.BP_BasicWater_C|SetAttackTimer _returnvalue_3 (.attacktimer _returnvalue_2)))
        (:Candle
          (bind _returnvalue_4 (Game|SpawnActorfromClass "/Game/Blueprints/Enemies/BP_Candle.BP_Candle_C" _returnvalue "Undefined" 0 0))
          (Variables|/Game/Blueprints/Enemies/BP_Candle.BP_Candle_C|SetDirection _returnvalue_4 (Math|Vector|GetForwardVector (Variables|Default|GetArrow)))
          (Variables|/Game/Blueprints/Enemies/BP_Candle.BP_Candle_C|SetHealth _returnvalue_4 (.health _returnvalue_2))
          (Variables|/Game/Blueprints/Enemies/BP_Candle.BP_Candle_C|SetSpeed _returnvalue_4 (.speed _returnvalue_2))
          (Variables|/Game/Blueprints/Enemies/BP_Candle.BP_Candle_C|SetEnemyDamage _returnvalue_4 (.damage _returnvalue_2))
          (Variables|/Game/Blueprints/Enemies/BP_Candle.BP_Candle_C|SetAttackTimer _returnvalue_4 (.attacktimer _returnvalue_2)))))))