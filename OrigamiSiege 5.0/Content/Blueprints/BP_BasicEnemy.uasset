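; BP_BasicEnemy is an enemy in a defense game that moves along a fixed direction and attacks defenses it overlaps.
; Overlapping a Defense stops movement and starts a looping AttackingDefense timer; Tick resumes movement once that target is invalid.
; Actor tags select the casts for damaging Archers or Guards and for taking Arrow damage from projectiles.
; At zero health, it leaves its detector's list, has GameManager update defenses, and is destroyed.
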(event EventBeginPlay)

(event Collision|EventActorBeginOverlap
  (params (OtherActor :type Actor%20Object%20Reference))
  (Utilities|FlowControl|Sequence
    (:then_0
      (if (Actor|ActorHasTag OtherActor "Defense")
        (Variables|Default|SetMoveEnabled false)
        (Variables|Default|SetAttackEnabled true)
        (Variables|Default|SetDefenseToAttackRef OtherActor)
        (Utilities|Time|SetTimerbyFunctionName 0 "AttackingDefense" 1.5 true)))
    (:then_1
      (if (Actor|ActorHasTag OtherActor "DefProjectile")
        (bind _array_element (Utilities|Array|ForEachLoopwithBreak (Variables|/Script/Engine.Actor|GetTags OtherActor) :!label _label)
          (:LoopBody
            (bind _correct (CallFunction|GetDamagebyProjectile OtherActor _array_element))
            (if _correct
              (goto _label Break)))
          (:Completed
            (Actor|DestroyActor OtherActor)))))))

(event EventTick
  (params (DeltaSeconds :type Float%20%28single-precision%29))
  (Utilities|FlowControl|Sequence
    (:then_0
      (if (Variables|Default|GetMoveEnabled)
        (Transformation|AddActorWorldOffset (* (Variables|Default|GetDirection) (* DeltaSeconds (Variables|Default|GetSpeed))))))
    (:then_1
      (if (<= (Variables|Default|GetHealth) 0.0)
        (CallFunction|EnemyDeath)
        (Actor|DestroyActor)))
    (:then_2
      (if (Variables|Default|GetAttackEnabled)
        (if (not (Utilities|IsValid (Variables|Default|GetDefenseToAttackRef)))
          (Variables|Default|SetMoveEnabled true)
          (Variables|Default|SetAttackEnabled false))))))

(fn ConstructionScript)

(fn EnemyDeath
  (bind _detectorref (Variables|Default|GetDetectorRef))
  (bind _returnvalue (Actor|GetActorOfClass "/Game/Blueprints/GameManager.GameManager_C"))
  (Utilities|Array|RemoveItem (Variables|/Game/Blueprints/BP_Detector.BP_Detector_C|GetEnemiesDetected _detectorref) self)
  (Default|UpdateDefenses _returnvalue _detectorref)
  (return))

(fn GetDamagebyProjectile
  (params (Projectile :type Actor%20Object%20Reference) (TagName :type Name))
  (switch name TagName
    (:Default
      (return false))
    (:Arrow
      (bind _asbp_arrow (Utilities|Casting|CastToBP_Arrow Projectile))
      (Variables|Default|SetHealth (- (Variables|Default|GetHealth) (Variables|/Game/Blueprints/BP_Arrow.BP_Arrow_C|GetArrowDamage _asbp_arrow)))
      (return true))))

(fn AttackingDefense
  (bind _enemydamage (Variables|Default|GetEnemyDamage))
  (bind _defensetoattackref (Variables|Default|GetDefenseToAttackRef))
  (if (Utilities|IsValid _defensetoattackref)
    (bind _array_element (Utilities|Array|ForEachLoopwithBreak (Variables|/Script/Engine.Actor|GetTags _defensetoattackref) :!label _label)
      (:LoopBody
        (switch name _array_element
          (:Archers
            (bind _asbp_archers (Utilities|Casting|CastToBP_Archers _defensetoattackref))
            (Default|GetDamagedbyEnemy _asbp_archers _enemydamage)
            (goto _label Break))
          (:Guard
            (bind _asbp_guard (Utilities|Casting|CastToBP_Guard _defensetoattackref))
            (Default|GetDamagedbyEnemy _asbp_guard _enemydamage)
            (goto _label Break))))
      (:Completed
        _)))
  (return))