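; BP_GridCell is a clickable grid tile for placing defenses, swapping its cube material while the cursor hovers over it.
; A left click spawns BP_Archers or BP_Guard slightly above the cell, according to the selection held by BP_GridManager.
; The new defense takes the cell's GridLine and registers with the matching line detector in GameManager.
; Grid snapping uses a zero grid size, so placement follows the cell's own position.
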(event EventBeginPlay
  (bind _returnvalue (Actor|GetActorOfClass "/Game/Blueprints/GameManager.GameManager_C"))
  (Variables|Default|SetGameManRef _returnvalue))

(event Collision|EventActorBeginOverlap
  (params (OtherActor :type Actor%20Object%20Reference)))

(event MouseInput|EventActorOnClicked
  (params (ButtonPressed :type Key%20Structure))
  (bind _returnvalue (Transformation|GetActorTransform))
  (bind (_location _rotation _scale) (Math|Transform|BreakTransform _returnvalue))
  (bind (_x _y _z) (Math|Vector|BreakVector _location))
  (if (== ButtonPressed "LeftMouseButton")
    (CallFunction|SwitchSpawnDefense (Math|Transform|MakeTransform (Math|Vector|MakeVector (Math|Float|SnapToGrid(Float) _x 0.0) (Math|Float|SnapToGrid(Float) _y 0.0) (+ _z 8e+01)) _rotation _scale))))

(event MouseInput|EventActorBeginCursorOver
  (Rendering|Material|SetMaterial (Variables|Default|GetCube) 0 "/Game/Materials/HoverMaterial.HoverMaterial"))

(event MouseInput|EventActorEndCursorOver
  (Rendering|Material|SetMaterial (Variables|Default|GetCube) 0 "/Game/Materials/BaseMaterial.BaseMaterial"))

(event EventTick
  (params (DeltaSeconds :type Float%20%28single-precision%29)))

(fn ConstructionScript)

(fn SwitchSpawnDefense
  (params (Transform :type Transform))
  (bind _gamemanref (Variables|Default|GetGameManRef))
  (bind _detectors (Variables|/Game/Blueprints/GameManager.GameManager_C|GetDetectors _gamemanref))
  (bind _returnvalue (Actor|GetActorOfClass "/Game/Blueprints/BP_GridManager.BP_GridManager_C"))
  (switch int (Variables|/Game/Blueprints/BP_GridManager.BP_GridManager_C|GetSelectedDefense _returnvalue)
    (:0
      (bind _returnvalue_2 (Game|SpawnActorfromClass "/Game/Blueprints/BP_Archers.BP_Archers_C" Transform "AlwaysSpawn" 0 0))
      (bind _output_get (Variables|/Game/Blueprints/BP_Archers.BP_Archers_C|SetDefenseLine _returnvalue_2 (Variables|Default|GetGridLine)))
      (Default|AddDefense (Utilities|Array|Get(acopy) _detectors _output_get) _returnvalue_2 (Variables|/Game/Blueprints/BP_GridManager.BP_GridManager_C|GetSelectedDefense _returnvalue)))
    (:1
      (bind _returnvalue_3 (Game|SpawnActorfromClass "/Game/Blueprints/BP_Guard.BP_Guard_C" Transform "AlwaysSpawn" 0 0))
      (bind _output_get_2 (Variables|/Game/Blueprints/BP_Guard.BP_Guard_C|SetDefenseLine _returnvalue_3 (Variables|Default|GetGridLine)))
      (Default|AddDefense (Utilities|Array|Get(acopy) _detectors _output_get_2) _returnvalue_3 (Variables|/Game/Blueprints/BP_GridManager.BP_GridManager_C|GetSelectedDefense _returnvalue))))
  (return))