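; Clickable construction grid cell that highlights on cursor hover and places the building selected in the GameManager.
; A left click builds a transform raised above the cell, calls SwitchSpawnBuilding, then triggers the manager's building notification check.
; SwitchSpawnBuilding looks up the Archery cost in a data table and, if affordable, spawns BP_BuildArchery, hands it the manager's Detectors, deducts Money and clears the selection.
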(event EventBeginPlay
  (bind _returnvalue (Actor|GetActorOfClass "/Game/Blueprints/GameManager.GameManager_C"))
  (Variables|Default|SetGameManRef _returnvalue))

(event Collision|EventActorBeginOverlap
  (params (OtherActor :type Actor%20Object%20Reference)))

(event EventTick
  (params (DeltaSeconds :type Float%20%28single-precision%29)))

(event MouseInput|EventActorBeginCursorOver
  (Rendering|Material|SetMaterial (Variables|Default|GetCube) 0 "/Game/Materials/HoverMaterial.HoverMaterial"))

(event MouseInput|EventActorEndCursorOver
  (Rendering|Material|SetMaterial (Variables|Default|GetCube) 0 "/Game/Materials/BaseMaterial.BaseMaterial"))

(event MouseInput|EventActorOnClicked
  (params (ButtonPressed :type Key%20Structure :default "None"))
  (bind _returnvalue (Transformation|GetActorTransform))
  (bind (_location _rotation _scale) (Math|Transform|BreakTransform _returnvalue))
  (bind (_x _y _z) (Math|Vector|BreakVector _location))
  (if (== ButtonPressed "LeftMouseButton")
    (CallFunction|SwitchSpawnBuilding (Math|Transform|MakeTransform (Math|Vector|MakeVector (Math|Float|SnapToGrid(Float) _x 0.0) (Math|Float|SnapToGrid(Float) _y 0.0) (+ _z 8e+01)) _rotation _scale))
    (Class|WPBP|CheckBuildingNotification(Message) (Variables|Default|GetGameManRef))))

(fn ConstructionScript)

(fn SwitchSpawnBuilding
  (params (Transform :type Transform))
  (bind _gamemanref (Variables|Default|GetGameManRef))
  (switch int (Variables|/Game/Blueprints/GameManager.GameManager_C|GetSelectedBuilding (Variables|Default|GetGameManRef))
    (:0
      (bind _returnvalue (Utilities|GetDataTableRow "/Game/Blueprints/Buildings/TypeBuildingsData.TypeBuildingsData" "Archery")
        (:then
          (if (>= (Variables|/Game/Blueprints/GameManager.GameManager_C|GetMoney _gamemanref) (.cost _returnvalue))
            (bind _returnvalue_2 (Game|SpawnActorfromClass "/Game/Blueprints/Buildings/BP_BuildArchery.BP_BuildArchery_C" Transform "Undefined" 0 0))
            (Variables|/Game/Blueprints/Buildings/BP_BuildArchery.BP_BuildArchery_C|SetDetectors _returnvalue_2 (Variables|/Game/Blueprints/GameManager.GameManager_C|GetDetectors (Variables|Default|GetGameManRef)))
            (Variables|/Game/Blueprints/GameManager.GameManager_C|SetMoney _gamemanref (- (Variables|/Game/Blueprints/GameManager.GameManager_C|GetMoney _gamemanref) (.cost _returnvalue)))
            (Variables|/Game/Blueprints/GameManager.GameManager_C|SetSelectedBuilding _gamemanref -1)
            (return)))))))