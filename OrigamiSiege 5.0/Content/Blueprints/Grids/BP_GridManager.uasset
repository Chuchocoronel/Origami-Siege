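; BP_GridManager is a grid manager actor that builds a grid of BP_GridCell actors when play begins.
; PopulateGrid clears GridArray, then uses nested loops over GridSizeX and GridSizeY to spawn cells spaced by WorldGridSize at a fixed height.
; Half-extent offsets center the grid on the world origin, with GridSizeY running along world X.
; Each cell stores its inner-loop index as GridLine and is added to GridArray.
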(event EventBeginPlay
  (CallFunction|PopulateGrid))

(event Collision|EventActorBeginOverlap
  (params (OtherActor :type Actor%20Object%20Reference)))

(event EventTick
  (params (DeltaSeconds :type Float%20%28single-precision%29)))

(fn ConstructionScript)

(fn PopulateGrid
  (bind _worldgridsize (Variables|Default|GetWorldGridSize))
  (bind _worldgridsize_2 (Variables|Default|GetWorldGridSize))
  (bind _worldgridsize_3 (Variables|Default|GetWorldGridSize))
  (Utilities|Array|Clear (Variables|Default|GetGridArray))
  (LocalVariables|SetWorldOffsetX (- (* (* (Variables|Default|GetGridSizeY) _worldgridsize_2) 0.5) (* _worldgridsize_2 0.5)))
  (LocalVariables|SetWorldOffsetY (- (* (* (Variables|Default|GetGridSizeX) _worldgridsize) 0.5) (* _worldgridsize 0.5)))
  (for _index (range 0 (- (Variables|Default|GetGridSizeX) 1))
    (for _index_2 (range 0 (- (Variables|Default|GetGridSizeY) 1))
      (bind _returnvalue (Game|SpawnActorfromClass "/Game/Blueprints/Grids/BP_GridCell.BP_GridCell_C" (Math|Transform|MakeTransform (Math|Vector|MakeVector (Math|Conversions|ToFloat(Integer) (- (* _index_2 _worldgridsize_3) (Math|Float|Truncate (LocalVariables|GetWorldOffsetX)))) (Math|Conversions|ToFloat(Integer) (- (* _worldgridsize_3 _index) (Math|Float|Truncate (LocalVariables|GetWorldOffsetY)))) 3e+01)) "AlwaysSpawn" 0 0))
      (Variables|/Game/Blueprints/Grids/BP_GridCell.BP_GridCell_C|SetGridLine _returnvalue _index_2)
      (Utilities|Array|Add (Variables|Default|GetGridArray) _returnvalue))))