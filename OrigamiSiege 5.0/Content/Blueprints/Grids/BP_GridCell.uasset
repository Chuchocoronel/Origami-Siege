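; Clickable grid cell that places the player's selected defense and swaps its cube material while the cursor hovers over it.
; A left click spawns an archer, guard, fire or bomb defense above the cell, based on the GameManager's selection, with stats from a data table.
; Each spawn registers with its grid line's detector and decrements that type's recruited count, then the selection resets.
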(event EventBeginPlay
  ;[1 1 1] Fill game manager variable
  (bind _returnvalue (Actor|GetActorOfClass "/Game/Blueprints/GameManager.GameManager_C"))
  (Variables|Default|SetGameManRef _returnvalue))

(event Collision|EventActorBeginOverlap
  (params (OtherActor :type Actor%20Object%20Reference)))

(event MouseInput|EventActorOnClicked
  (params (ButtonPressed :type Key%20Structure :default "None"))
  (bind _returnvalue (Transformation|GetActorTransform))
  (bind (_location _rotation _scale) (Math|Transform|BreakTransform _returnvalue))
  (bind (_x _y _z) (Math|Vector|BreakVector _location))
  ;[1 1 1] Spawn defense in the grid
  (if (== ButtonPressed "LeftMouseButton")
    (CallFunction|SwitchSpawnDefense (Math|Transform|MakeTransform (Math|Vector|MakeVector (Math|Float|SnapToGrid(Float) _x 0.0) (Math|Float|SnapToGrid(Float) _y 0.0) (+ _z 8e+01)) _rotation _scale))
    (Class|WPBP|CheckNotificationRecuited(Message) (Variables|Default|GetGameManRef))))

(event MouseInput|EventActorBeginCursorOver
  ;[1 1 1] Change colors when cursor over
  (Rendering|Material|SetMaterial (Variables|Default|GetCube) 0 "/Game/Materials/HoverMaterial.HoverMaterial"))

(event MouseInput|EventActorEndCursorOver
  ;[1 1 1] Change colors when cursor over
  (Rendering|Material|SetMaterial (Variables|Default|GetCube) 0 "/Game/Materials/BaseMaterial.BaseMaterial"))

(event EventTick
  (params (DeltaSeconds :type Float%20%28single-precision%29)))

(fn ConstructionScript)

(fn SwitchSpawnDefense
  (params (Transform :type Transform))
  (bind _gamemanref (Variables|Default|GetGameManRef))
  (bind _gridline (Variables|Default|GetGridLine))
  (bind _gamemanref_2 (Variables|Default|GetGameManRef))
  (bind _detectors (Variables|/Game/Blueprints/GameManager.GameManager_C|GetDetectors _gamemanref))
  (bind _output (Utilities|Array|Get(acopy) _detectors _gridline))
  (switch int (Variables|/Game/Blueprints/GameManager.GameManager_C|GetSelectedDefense _gamemanref_2)
    (:Default
      _)
    (:0
      (bind _returnvalue (Utilities|GetDataTableRow "/Game/Blueprints/Defenses/TypeDefensesData.TypeDefensesData" "Archer")
        (:then
          (bind _returnvalue_2 (Game|SpawnActorfromClass "/Game/Blueprints/Defenses/BP_Archers.BP_Archers_C" Transform "AlwaysSpawn" 0 0))
          (Variables|/Game/Blueprints/Defenses/BP_Archers.BP_Archers_C|SetCost _returnvalue_2 (.cost _returnvalue))
          (Variables|/Game/Blueprints/Defenses/BP_Archers.BP_Archers_C|SetHealth _returnvalue_2 (.health _returnvalue))
          (Variables|/Game/Blueprints/Defenses/BP_Archers.BP_Archers_C|SetAttackTimer _returnvalue_2 (.attacktimer _returnvalue))
          (Variables|/Game/Blueprints/Defenses/BP_Archers.BP_Archers_C|SetDamage _returnvalue_2 (.damage _returnvalue))
          (Variables|/Game/Blueprints/Defenses/BP_Archers.BP_Archers_C|SetSpeed _returnvalue_2 (.speed _returnvalue))
          (Default|AddDefense _output _returnvalue_2 (Variables|/Game/Blueprints/GameManager.GameManager_C|GetSelectedDefense _gamemanref_2))
          (Variables|/Game/Blueprints/GameManager.GameManager_C|SetRecuitedArchers _gamemanref (- (Variables|/Game/Blueprints/GameManager.GameManager_C|GetRecuitedArchers _gamemanref) 1)))))
    (:1
      (bind _returnvalue_3 (Utilities|GetDataTableRow "/Game/Blueprints/Defenses/TypeDefensesData.TypeDefensesData" "Guard")
        (:then
          (bind _returnvalue_4 (Game|SpawnActorfromClass "/Game/Blueprints/Defenses/BP_Guard.BP_Guard_C" Transform "AlwaysSpawn" 0 0))
          (Variables|/Game/Blueprints/Defenses/BP_Guard.BP_Guard_C|SetCost _returnvalue_4 (.cost _returnvalue_3))
          (Variables|/Game/Blueprints/Defenses/BP_Guard.BP_Guard_C|SetHealth _returnvalue_4 (.health _returnvalue_3))
          (Variables|/Game/Blueprints/Defenses/BP_Guard.BP_Guard_C|SetAttackTimer _returnvalue_4 (.attacktimer _returnvalue_3))
          (Variables|/Game/Blueprints/Defenses/BP_Guard.BP_Guard_C|SetSpeed _returnvalue_4 (.speed _returnvalue_3))
          (Default|AddDefense _output _returnvalue_4 (Variables|/Game/Blueprints/GameManager.GameManager_C|GetSelectedDefense _gamemanref_2))
          (Variables|/Game/Blueprints/GameManager.GameManager_C|SetRecuitedGuards _gamemanref (- (Variables|/Game/Blueprints/GameManager.GameManager_C|GetRecuitedGuards _gamemanref) 1)))))
    (:2
      (bind _returnvalue_5 (Utilities|GetDataTableRow "/Game/Blueprints/Defenses/TypeDefensesData.TypeDefensesData" "Fire")
        (:then
          (bind _returnvalue_6 (Game|SpawnActorfromClass "/Game/Blueprints/Defenses/BP_Fire.BP_Fire_C" Transform "AlwaysSpawn" 0 0))
          (Variables|/Game/Blueprints/Defenses/BP_Fire.BP_Fire_C|SetCost _returnvalue_6 (.cost _returnvalue_5))
          (Variables|/Game/Blueprints/Defenses/BP_Fire.BP_Fire_C|SetHealth _returnvalue_6 (.health _returnvalue_5))
          (Variables|/Game/Blueprints/Defenses/BP_Fire.BP_Fire_C|SetAttackTimer _returnvalue_6 (.attacktimer _returnvalue_5))
          (Variables|/Game/Blueprints/Defenses/BP_Fire.BP_Fire_C|SetDamage _returnvalue_6 (.damage _returnvalue_5))
          (Variables|/Game/Blueprints/Defenses/BP_Fire.BP_Fire_C|SetSpeed _returnvalue_6 (.speed _returnvalue_5))
          (Default|AddDefense _output _returnvalue_6 (Variables|/Game/Blueprints/GameManager.GameManager_C|GetSelectedDefense _gamemanref_2))
          (Variables|/Game/Blueprints/GameManager.GameManager_C|SetRecuitedFires _gamemanref (- (Variables|/Game/Blueprints/GameManager.GameManager_C|GetRecuitedFires _gamemanref) 1)))))
    (:3
      (bind _returnvalue_7 (Utilities|GetDataTableRow "/Game/Blueprints/Defenses/TypeDefensesData.TypeDefensesData" "Bomb")
        (:then
          (bind _returnvalue_8 (Game|SpawnActorfromClass "/Game/Blueprints/Defenses/BP_Bomb.BP_Bomb_C" Transform "AlwaysSpawn" 0 0))
          (Variables|/Game/Blueprints/Defenses/BP_Bomb.BP_Bomb_C|SetCost _returnvalue_8 (.cost _returnvalue_7))
          (Variables|/Game/Blueprints/Defenses/BP_Bomb.BP_Bomb_C|SetHealth _returnvalue_8 (.health _returnvalue_7))
          (Variables|/Game/Blueprints/Defenses/BP_Bomb.BP_Bomb_C|SetAttackTimer _returnvalue_8 (.attacktimer _returnvalue_7))
          (Variables|/Game/Blueprints/Defenses/BP_Bomb.BP_Bomb_C|SetDamage _returnvalue_8 (.damage _returnvalue_7))
          (Variables|/Game/Blueprints/Defenses/BP_Bomb.BP_Bomb_C|SetSpeed _returnvalue_8 (.speed _returnvalue_7))
          (Default|AddDefense _output _returnvalue_8 (Variables|/Game/Blueprints/GameManager.GameManager_C|GetSelectedDefense _gamemanref_2))
          (Variables|/Game/Blueprints/GameManager.GameManager_C|SetRecuitedBombs _gamemanref (- (Variables|/Game/Blueprints/GameManager.GameManager_C|GetRecuitedBombs _gamemanref) 1))))))
  (Variables|/Game/Blueprints/GameManager.GameManager_C|SetSelectedDefense _gamemanref_2 -1)
  (return))