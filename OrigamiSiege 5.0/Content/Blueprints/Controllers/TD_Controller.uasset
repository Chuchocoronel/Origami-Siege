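; TD_Controller is a player controller for a top-down camera, showing the cursor and enabling click and mouse-over events.
; On BeginPlay it caches the CameraPawn, which the MoveHorizontal axis slides along its local Y.
; Pan speed scales with spring arm length, clamped, times MoveSensitivity.
; Tick computes horizontal screen-edge scroll from cursor position, but the offset node that would apply it is disconnected.
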(event EventBeginPlay
  (Utilities|CastReferences
    (:ReturnNode
      (Variables|Default|SetbEnableClickEvents true)
      (Variables|Default|SetbEnableMouseOverEvents true)
      (Variables|Default|SetbShowMouseCursor true))))

(event EventTick
  (params (DeltaSeconds :type Float%20%28single-precision%29))
  (bind _deltaxspeed (Utilities|ScreenEdgeMovement)))

(event Input|AxisEvents|InputAxisMoveHorizontal
  (params (AxisValue :type Float%20%28single-precision%29))
  (bind _cameraref (Variables|Default|GetCameraRef))
  (Transformation|SetActorTransform _cameraref (Utilities|CamMovementX AxisValue (CallFunction|MovementSpeedCalculation) (Variables|Default|GetMoveSensitivity) _cameraref)))

(fn ConstructionScript)

(fn MovementSpeedCalculation
  (return (Math|Float|Clamp(Float) (/ (Variables|/Script/Engine.SpringArmComponent|GetTargetArmLength (Variables|/Game/Blueprints/Controllers/CameraPawn.CameraPawn_C|GetSpringArm (Variables|Default|GetCameraRef))) 1e+02) 5.0 2e+01)))