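; BP_BasicWater is an enemy that moves along a set direction and attacks defenses in its path.
; Overlapping a "Defense"-tagged actor stops movement and starts a looping damage timer, with movement resuming once that defense is invalid.
; At zero health it leaves its detector's list, updates GameManager's defenses, money and messages, then destroys itself.
; The tag-and-cast AttackingDefense function is not called here; attacks use ApplyDamage.
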(event Custom|AttackDefense
  ;[1 1 1] Attack defense when contact
  (Game|Damage|ApplyDamage (stale Collision|EventActorBeginOverlap _output_get) (Variables|Default|GetEnemyDamage) 0 0)
  (if (not (Utilities|IsValid (Variables|Default|GetDefenseToAttackRef)))
    (Variables|Default|SetMoveEnabled true)))

(event EventBeginPlay)

(event Collision|EventActorBeginOverlap
  (params (OtherActor :type Actor%20Object%20Reference))
  (Utilities|FlowControl|Sequence
    (:then_0
      ;[1 1 1] Attack defense when contact
      (if (Actor|ActorHasTag OtherActor "Defense")
        (Variables|Default|SetMoveEnabled false)
        (bind _output_get (Variables|Default|SetDefenseToAttackRef OtherActor))
        (Utilities|Time|SetTimerbyEvent (delegate Custom|AttackDefense) (Variables|Default|GetAttackTimer) true)))))

(event EventTick
  (params (DeltaSeconds :type Float%20%28single-precision%29))
  ;[1 1 1] Movement
  (Utilities|FlowControl|Sequence
    (:then_0
      (if (Variables|Default|GetMoveEnabled)
        (Transformation|AddActorWorldOffset (* (Variables|Default|GetDirection) (* DeltaSeconds (Variables|Default|GetSpeed))))))))

(event Game|Damage|EventAnyDamage
  (params (Damage :type Float%20%28single-precision%29) (DamageType :type Damage%20Type%20Object%20Reference) (InstigatedBy :type Controller%20Object%20Reference) (DamageCauser :type Actor%20Object%20Reference))
  ;[1 1 1] Get damaged and death
  (CallFunction|GetDamaged Damage)
  (if (<= (Variables|Default|GetHealth) 0.0)
    (CallFunction|EnemyDeath)
    (Actor|DestroyActor)))

(fn ConstructionScript)

(fn EnemyDeath
  (bind _detectorref (Variables|Default|GetDetectorRef))
  (bind _returnvalue (Actor|GetActorOfClass "/Game/Blueprints/GameManager.GameManager_C"))
  (Utilities|Array|RemoveItem (Variables|/Game/Blueprints/LvlComponents/BP_Detector.BP_Detector_C|GetEnemiesDetected _detectorref) self)
  (Default|UpdateDefenses _returnvalue _detectorref)
  (Variables|/Game/Blueprints/GameManager.GameManager_C|SetMoney _returnvalue (+ (Variables|/Game/Blueprints/GameManager.GameManager_C|GetMoney _returnvalue) (Variables|Default|GetDeathMoney)))
  (Class|WPBP|CheckNotificationMoney(Message) _returnvalue)
  (Class|WPBP|EnemyLess(Message) _returnvalue)
  (return))

(fn GetDamaged
  (params (Defense%20Damage :type Float%20%28double-precision%29))
  (Variables|Default|SetHealth (- (Variables|Default|GetHealth) Defense%20Damage))
  (return))

(fn AttackingDefense
  (bind _enemydamage (Variables|Default|GetEnemyDamage))
  (bind _defensetoattackref (Variables|Default|GetDefenseToAttackRef))
  (if (Utilities|IsValid _defensetoattackref)
    (bind _array_element (Utilities|Array|ForEachLoopwithBreak (Variables|/Script/Engine.Actor|GetTags _defensetoattackref) :!label _label)
      (:LoopBody
        (switch name _array_element
          (:Archers
            (bind _asbp_archers (Utilities|Casting|CastToBP_Archers _defensetoattackref))
            (Default|GetDamagedbyEnemy _asbp_archers _enemydamage)
            (goto _label Break))
          (:Guard
            (bind _asbp_guard (Utilities|Casting|CastToBP_Guard _defensetoattackref))
            (Default|GetDamagedbyEnemy _asbp_guard _enemydamage)
            (goto _label Break))))
      (:Completed
        _)))
  (return))