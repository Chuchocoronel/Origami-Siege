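; BP_Knife is a spinning knife actor, filed under Enemies, that damages actors tagged "Defense".
; A fast looping timer started on BeginPlay rotates the Knife component in world space, in place of using Tick.
; Overlapping a "Defense" actor applies its Damage value without destroying the knife, which is destroyed only when it hits an actor tagged "Floor".
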(event Custom|Spin
  (Transformation|AddWorldRotation (Variables|Default|GetKnife) "0.000000,0.000000,-5.000000" false false))

(event EventBeginPlay
  (Utilities|Time|SetTimerbyEvent (delegate Custom|Spin) 0.01 true))

(event Collision|EventActorBeginOverlap
  (params (OtherActor :type Actor%20Object%20Reference))
  ;[1 1 1] Apply damage to enemy
  (if (Actor|ActorHasTag OtherActor "Defense")
    (Game|Damage|ApplyDamage OtherActor (Variables|Default|GetDamage) 0 self)))

(event EventTick
  (params (DeltaSeconds :type Float%20%28single-precision%29)))

(event Collision|EventActorEndOverlap
  (params (OtherActor :type Actor%20Object%20Reference)))

(event Collision|EventHit
  (params (MyComp :type Primitive%20Component%20Object%20Reference) (Other :type Actor%20Object%20Reference) (OtherComp :type Primitive%20Component%20Object%20Reference) (bSelfMoved :type Boolean) (HitLocation :type Vector :default "0, 0, 0") (HitNormal :type Vector :default "0, 0, 0") (NormalImpulse :type Vector :default "0, 0, 0") (Hit :type Hit%20Result%20Structure%20%28by%20ref%29))
  (if (Actor|ActorHasTag Other "Floor")
    (Actor|DestroyActor)))

(fn ConstructionScript)