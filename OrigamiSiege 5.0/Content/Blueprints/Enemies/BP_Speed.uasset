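; BP_Speed is a wheel enemy that moves along a set direction and attacks defenses blocking it.
; Tagged collider overlaps either halt it and queue the defense for timed damage, resuming once none remain, or deal it delayed explosion damage.
; Hits trigger sound and a brief material flash.
; Death removes it from its detector, updates defenses through GameManager, awards money and destroys the actor.
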(event OnComponentBeginOverlap(Collider)
  (params (OverlappedComponent :type Primitive%20Component%20Object%20Reference) (OtherActor :type Actor%20Object%20Reference) (OtherComp :type Primitive%20Component%20Object%20Reference) (OtherBodyIndex :type Integer) (bFromSweep :type Boolean) (SweepResult :type Hit%20Result%20Structure%20%28by%20ref%29))
  (if (Actor|ActorHasTag OtherActor "Defense")
    (if (Components|ComponentHasTag OtherComp "Stop")
      (Utilities|Array|AddUnique (Variables|Default|GetDefenseToAttackRef) OtherActor)
      (Variables|Default|SetMoveEnabled false)
      (elif (Components|ComponentHasTag OtherComp "Explosion")
        (Utilities|FlowControl|Delay 0.3)
        (Game|Damage|ApplyDamage self 1e+02 0 0)))))

(event OnComponentEndOverlap(Collider)
  (params (OverlappedComponent :type Primitive%20Component%20Object%20Reference) (OtherActor :type Actor%20Object%20Reference) (OtherComp :type Primitive%20Component%20Object%20Reference) (OtherBodyIndex :type Integer))
  (if (Actor|ActorHasTag OtherActor "Defense")
    (if (Components|ComponentHasTag OtherComp "Stop")
      (Utilities|Array|RemoveItem (Variables|Default|GetDefenseToAttackRef) OtherActor)
      (if (not (> (Utilities|Array|Length (Variables|Default|GetDefenseToAttackRef)) 0))
        (Variables|Default|SetMoveEnabled true)))))

(event Custom|AttackDefense
  (bind _defensetoattackref (Variables|Default|GetDefenseToAttackRef))
  (if (> (Utilities|Array|Length _defensetoattackref) 0)
    (Game|Damage|ApplyDamage (Utilities|Array|Get(acopy) _defensetoattackref) (Variables|Default|GetEnemyDamage) 0 self)))

(event Custom|HirMat
  (bind _skeletalmesh (Variables|Default|GetSkeletalMesh))
  (Rendering|Material|SetMaterial _skeletalmesh 4 "/Game/Models/Enemies/Wheel/Body.Body")
  (Rendering|Material|SetMaterial _skeletalmesh 5 "/Game/Models/Enemies/Wheel/Spike.Spike")
  (Rendering|Material|SetMaterial _skeletalmesh 3 "/Game/Models/Enemies/Eyelid.Eyelid"))

(event EventBeginPlay
  (Components|Animation|PlayAnimation (Variables|Default|GetSkeletalMesh) "/Game/Models/Enemies/Wheel/Wheel_Attack_Anim.Wheel_Attack_Anim" true)
  (Utilities|Time|SetTimerbyEvent (delegate Custom|AttackDefense) (Variables|Default|GetAttackTimer) true))

(event Collision|EventActorBeginOverlap
  (params (OtherActor :type Actor%20Object%20Reference)))

(event EventTick
  (params (DeltaSeconds :type Float%20%28single-precision%29))
  ;[1 1 1] Movement
  (Utilities|FlowControl|Sequence
    (:then_0
      (if (Variables|Default|GetMoveEnabled)
        (Transformation|AddActorWorldOffset (* (Variables|Default|GetDirection) (* DeltaSeconds (Variables|Default|GetSpeed))))))))

(event Collision|EventActorEndOverlap
  (params (OtherActor :type Actor%20Object%20Reference)))

(event Game|Damage|EventAnyDamage
  (params (Damage :type Float%20%28single-precision%29) (DamageType :type Damage%20Type%20Object%20Reference) (InstigatedBy :type Controller%20Object%20Reference) (DamageCauser :type Actor%20Object%20Reference))
  (bind _skeletalmesh (Variables|Default|GetSkeletalMesh))
  ;[1 1 1] Get damaged and death
  (CallFunction|GetDamaged Damage)
  (Audio|PlaySoundatLocation "/Game/Music/Enemy_hit.Enemy_hit" (Transformation|GetActorLocation) "0, 0, 0" 1.0 1.0 0.0 "/Game/Music/Attenuation.Attenuation" 0 0 0)
  (Rendering|Material|SetMaterial _skeletalmesh 3 "/Game/Models/Enemies/Hit.Hit")
  (Rendering|Material|SetMaterial _skeletalmesh 4 "/Game/Models/Enemies/Hit.Hit")
  (Rendering|Material|SetMaterial _skeletalmesh 5 "/Game/Models/Enemies/Hit.Hit")
  (Utilities|Time|SetTimerbyEvent (delegate Custom|HirMat) 0.2)
  (if (<= (Variables|Default|GetHealth) 0.0)
    (CallFunction|EnemyDeath)
    (Audio|PlaySoundatLocation "/Game/Music/Wheel_death.Wheel_death" (Transformation|GetActorLocation) "0, 0, 0" 1.0 1.0 0.0 "/Game/Music/Attenuation.Attenuation" 0 0 0)
    (Actor|DestroyActor)))

(fn ConstructionScript)

(fn EnemyDeath
  (bind _detectorref (Variables|Default|GetDetectorRef))
  (bind _returnvalue (Actor|GetActorOfClass "/Game/Blueprints/GameManager.GameManager_C"))
  (Utilities|Array|RemoveItem (Variables|/Game/Blueprints/LvlComponents/BP_Detector.BP_Detector_C|GetEnemiesDetected _detectorref) self)
  (Default|UpdateDefenses _returnvalue _detectorref)
  (Variables|/Game/Blueprints/GameManager.GameManager_C|SetMoney _returnvalue (+ (Variables|/Game/Blueprints/GameManager.GameManager_C|GetMoney _returnvalue) (Variables|Default|GetDeathMoney)))
  (Class|WPBP|CheckNotificationMoney(Message) _returnvalue)
  (Class|WPBP|EnemyLess(Message) _returnvalue)
  (return))

(fn GetDamaged
  (params (Defense%20Damage :type Float%20%28double-precision%29))
  (Variables|Default|SetHealth (- (Variables|Default|GetHealth) Defense%20Damage))
  (return))