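; BP_Archers is an archer actor that fires arrows while enemies are in its EnemyList and can be killed by enemy damage.
; Tick runs an AttackTimer countdown that calls AttackEnemy to spawn a BP_Arrow at ShotPoint's transform, without passing it a target.
; GetDamagedByEnemy subtracts from Health, and Tick destroys the actor once Health reaches zero.
; Nothing in these graphs fills or prunes EnemyList.
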(event EventBeginPlay)

(event Collision|EventActorBeginOverlap
  (params (OtherActor :type Actor%20Object%20Reference)))

(event EventTick
  (params (DeltaSeconds :type Float%20%28single-precision%29))
  (Utilities|FlowControl|Sequence
    (:then_0
      (if (>= (Utilities|Array|Length (Variables|Default|GetEnemyList)) 1)
        (bind _output_get (Variables|Default|SetTimer (- (Variables|Default|GetTimer) DeltaSeconds)))
        (if (<= _output_get 0.0)
          (Variables|Default|SetTimer (Variables|Default|GetAttackTimer))
          (CallFunction|AttackEnemy))))
    (:then_1
      (if (<= (Variables|Default|GetHealth) 0.0)
        (Actor|DestroyActor)))))

(fn ConstructionScript)

(fn AttackEnemy
  (if (!= (Utilities|Array|Length (Variables|Default|GetEnemyList)) 0)
    (Game|SpawnActorfromClass "/Game/Blueprints/BP_Arrow.BP_Arrow_C" (Transformation|GetWorldTransform (Variables|Default|GetShotPoint)) "Undefined" 0 0)))

(fn GetDamagedbyEnemy
  (params (EnemyDamage :type Float%20%28double-precision%29))
  (Variables|Default|SetHealth (- (Variables|Default|GetHealth) EnemyDamage))
  (return))