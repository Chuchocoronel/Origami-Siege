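; BP_Archers is a defense unit of three archers that marches along +Y to a slightly randomized line, pausing while overlapping an enemy's EStop component.
; While EnemyList has entries, a Tick countdown spawns BP_Arrow at ShotPoint with the unit's damage.
; Damage reduces health and briefly swaps all three archers to a hit material.
; At zero health it removes itself from DetectorRef's DefendersLine and is destroyed.
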(event OnComponentBeginOverlap(Collider)
  (params (OverlappedComponent :type Primitive%20Component%20Object%20Reference) (OtherActor :type Actor%20Object%20Reference) (OtherComp :type Primitive%20Component%20Object%20Reference) (OtherBodyIndex :type Integer) (bFromSweep :type Boolean) (SweepResult :type Hit%20Result%20Structure%20%28by%20ref%29))
  (if (Actor|ActorHasTag OtherActor "Enemy")
    (if (Components|ComponentHasTag OtherComp "EStop")
      (Variables|Default|SetCanMove false))))

(event OnComponentEndOverlap(Collider)
  (params (OverlappedComponent :type Primitive%20Component%20Object%20Reference) (OtherActor :type Actor%20Object%20Reference) (OtherComp :type Primitive%20Component%20Object%20Reference) (OtherBodyIndex :type Integer))
  (if (Actor|ActorHasTag OtherActor "Enemy")
    (if (Components|ComponentHasTag OtherComp "EStop")
      (Variables|Default|SetCanMove true))))

(event Custom|HitMat
  (Rendering|Material|SetMaterial (Variables|Default|GetArcher1) 0 "/Game/Materials/DefaultMaterial.DefaultMaterial"))

(event EventBeginPlay
  (Variables|Default|SetPosition (+ (Math|Random|RandomFloatinRange -2e+01 2e+01) -8.6e+02)))

(event Collision|EventActorBeginOverlap
  (params (OtherActor :type Actor%20Object%20Reference)))

(event EventTick
  (params (DeltaSeconds :type Float%20%28single-precision%29))
  (Utilities|FlowControl|Sequence
    (:then_0
      ;[1 1 1] Attack enemies when detected
      (if (>= (Utilities|Array|Length (Variables|Default|GetEnemyList)) 1)
        (bind _output_get (Variables|Default|SetTimer (- (Variables|Default|GetTimer) DeltaSeconds)))
        (if (<= _output_get 0.0)
          (Variables|Default|SetTimer (Variables|Default|GetAttackTimer))
          (CallFunction|AttackEnemy))))
    (:then_1
      (if (Variables|Default|GetCanMove)
        (if (< (.y (Transformation|GetActorLocation)) (Variables|Default|GetPosition))
          (Transformation|AddActorWorldOffset (* "0,1.000000,0" (* DeltaSeconds (Variables|Default|GetSpeed)))))))))

(event Game|Damage|EventAnyDamage
  (params (Damage :type Float%20%28single-precision%29) (DamageType :type Damage%20Type%20Object%20Reference) (InstigatedBy :type Controller%20Object%20Reference) (DamageCauser :type Actor%20Object%20Reference))
  ;[1 1 1] Get damaged and death
  (CallFunction|GetDamagedbyEnemy Damage)
  (Rendering|Material|SetMaterial (Variables|Default|GetArcher1) 0 "/Game/Materials/HitMaterial.HitMaterial")
  (Utilities|Time|SetTimerbyEvent (delegate Custom|HitMat) 0.2)
  (if (<= (Variables|Default|GetHealth) 0.0)
    (CallFunction|DefenseDeath)
    (Actor|DestroyActor)))

(event Collision|EventActorEndOverlap
  (params (OtherActor :type Actor%20Object%20Reference)))

(fn ConstructionScript)

(fn AttackEnemy
  (if (!= (Utilities|Array|Length (Variables|Default|GetEnemyList)) 0)
    (bind _returnvalue (Game|SpawnActorfromClass "/Game/Blueprints/Defenses/BP_Arrow.BP_Arrow_C" (Transformation|GetWorldTransform (Variables|Default|GetShotPoint)) "Undefined" 0 0))
    (Variables|/Game/Blueprints/Defenses/BP_Arrow.BP_Arrow_C|SetDamage _returnvalue (Variables|Default|GetDamage))))

(fn GetDamagedbyEnemy
  (params (EnemyDamage :type Float%20%28double-precision%29))
  (Variables|Default|SetHealth (- (Variables|Default|GetHealth) EnemyDamage))
  (return))

(fn DefenseDeath
  (Utilities|Array|RemoveItem (Variables|/Game/Blueprints/LvlComponents/BP_Detector.BP_Detector_C|GetDefendersLine (Variables|Default|GetDetectorRef)) self)
  (return))