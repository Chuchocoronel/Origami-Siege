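; BP_Bomb is a walking suicide-bomber defense, animated with Paper2D flipbooks, that advances along +Y with a random X offset and limited lifespan.
; Overlapping an enemy's EStop-tagged component stops it, plays the attack animation, enables explosion overlaps, spawns an Explosion actor and shortens its lifespan.
; Damage reduces health with a hit sound and red flash; at zero health it leaves its detector's DefendersLine and is destroyed.
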(event OnComponentBeginOverlap(Collider)
  (params (OverlappedComponent :type Primitive%20Component%20Object%20Reference) (OtherActor :type Actor%20Object%20Reference) (OtherComp :type Primitive%20Component%20Object%20Reference) (OtherBodyIndex :type Integer) (bFromSweep :type Boolean) (SweepResult :type Hit%20Result%20Structure%20%28by%20ref%29))
  (if (Actor|ActorHasTag OtherActor "Enemy")
    (if (Components|ComponentHasTag OtherComp "EStop")
      (Variables|/Script/Engine.PrimitiveComponent|SetbGenerateOverlapEvents (Variables|Default|GetExplosion) true)
      (Variables|Default|SetCanMove false)
      (Actor|SetLifeSpan 0.3)
      (Sprite|SetFlipbook (Variables|Default|GetBomb_Anim) "/Game/Models/Defenses/Bomb/Attack/Bombman_Attack_Anim.Bombman_Attack_Anim")
      (Game|SpawnActorfromClass "/Game/Models/Defenses/Bomb/Explosion/Explosion.Explosion_C" (Transformation|GetActorTransform self) "AlwaysSpawn" 0 0))))

(event Custom|HitMat
  (Sprite|SetSpriteColor (Variables|Default|GetBomb_Anim) "(R=1.000000,G=1.000000,B=1.000000,A=1.000000)"))

(event EventBeginPlay
  (Actor|SetLifeSpan 2e+01)
  (Transformation|AddActorWorldOffset (Math|Vector|MakeVector (Math|Random|RandomFloatinRange -5e+01 5e+01) 0.0 0.0))
  (Sprite|SetFlipbook (Variables|Default|GetBomb_Anim) "/Game/Models/Defenses/Bomb/Walk/Bombman_Walk_Anim.Bombman_Walk_Anim"))

(event EventTick
  (params (DeltaSeconds :type Float%20%28single-precision%29))
  (if (Variables|Default|GetCanMove)
    (Transformation|AddActorWorldOffset (* "0,1.000000,0" (* DeltaSeconds (Variables|Default|GetSpeed))))))

(event Game|Damage|EventAnyDamage
  (params (Damage :type Float%20%28single-precision%29) (DamageType :type Damage%20Type%20Object%20Reference) (InstigatedBy :type Controller%20Object%20Reference) (DamageCauser :type Actor%20Object%20Reference))
  (CallFunction|GetDamagedbyEnemy Damage)
  (Audio|SpawnSoundatLocation "/Game/Music/Defense_hit.Defense_hit" (Transformation|GetActorLocation) "0, 0, 0" 1.0 1.0 0.0 "/Game/Music/Attenuation.Attenuation" 0)
  (Sprite|SetSpriteColor (Variables|Default|GetBomb_Anim) "(R=1.000000,G=0.000000,B=0.000000,A=1.000000)")
  (Utilities|Time|SetTimerbyEvent (delegate Custom|HitMat) 0.2)
  (if (<= (Variables|Default|GetHealth) 0.0)
    (CallFunction|DefenseDeath)
    (Actor|DestroyActor)))

(fn ConstructionScript)

(fn GetDamagedbyEnemy
  (params (EnemyDamage :type Float%20%28double-precision%29))
  (Variables|Default|SetHealth (- (Variables|Default|GetHealth) EnemyDamage))
  (return))

(fn DefenseDeath
  (Utilities|Array|RemoveItem (Variables|/Game/Blueprints/LvlComponents/BP_Detector.BP_Detector_C|GetDefendersLine (Variables|Default|GetDetectorRef)) self)
  (return))