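; BP_Fire is a fireman defender that walks along +Y to a slightly randomized stop position, switching between walk and idle flipbooks.
; Overlapping an enemy's EStop component halts it, and it resumes when that overlap ends short of its position.
; A looping timer drains its health through self-damage.
; Hits flash the sprite red, and at zero health it leaves the detector's DefendersLine and is destroyed.
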(event OnComponentBeginOverlap(Collider)
  (params (OverlappedComponent :type Primitive%20Component%20Object%20Reference) (OtherActor :type Actor%20Object%20Reference) (OtherComp :type Primitive%20Component%20Object%20Reference) (OtherBodyIndex :type Integer) (bFromSweep :type Boolean) (SweepResult :type Hit%20Result%20Structure%20%28by%20ref%29))
  (if (Actor|ActorHasTag OtherActor "Enemy")
    (if (Components|ComponentHasTag OtherComp "EStop")
      (Variables|Default|SetCanMove false))))

(event OnComponentEndOverlap(Collider)
  (params (OverlappedComponent :type Primitive%20Component%20Object%20Reference) (OtherActor :type Actor%20Object%20Reference) (OtherComp :type Primitive%20Component%20Object%20Reference) (OtherBodyIndex :type Integer))
  (if (Actor|ActorHasTag OtherActor "Enemy")
    (if (Components|ComponentHasTag OtherComp "EStop")
      (if (< (.y (Transformation|GetActorLocation)) (Variables|Default|GetPosition))
        (Variables|Default|SetCanMove true)))))

(event Custom|LoseHealth
  (bind _self self)
  (Game|Damage|ApplyDamage _self 1.0 0 _self))

(event Custom|HitMat
  (Sprite|SetSpriteColor (Variables|Default|GetFireman_Anim) "(R=1.000000,G=1.000000,B=1.000000,A=1.000000)"))

(event EventBeginPlay
  (Variables|Default|SetPosition (+ (Math|Random|RandomFloatinRange -2e+01 2e+01) -3e+02))
  (Utilities|Time|SetTimerbyEvent (delegate Custom|LoseHealth) 1.0 true)
  (Transformation|AddActorWorldOffset (Math|Vector|MakeVector (Math|Random|RandomFloatinRange -5e+01 5e+01) 0.0 0.0))
  (Sprite|SetFlipbook (Variables|Default|GetFireman_Anim) "/Game/Models/Defenses/Fire/Walk/Fireman_Walk_Anim.Fireman_Walk_Anim"))

(event Collision|EventActorBeginOverlap
  (params (OtherActor :type Actor%20Object%20Reference)))

(event EventTick
  (params (DeltaSeconds :type Float%20%28single-precision%29))
  (bind _fireman_anim (Variables|Default|GetFireman_Anim))
  (if (Variables|Default|GetCanMove)
    (if (< (.y (Transformation|GetActorLocation)) (Variables|Default|GetPosition))
      (Transformation|AddActorWorldOffset (* "0,1.000000,0" (* DeltaSeconds (Variables|Default|GetSpeed))))
      (Sprite|SetFlipbook _fireman_anim "/Game/Models/Defenses/Fire/Walk/Fireman_Walk_Anim.Fireman_Walk_Anim")
      (else
        (Variables|Default|SetCanMove false)))
    (else
      (Sprite|SetFlipbook _fireman_anim "/Game/Models/Defenses/Fire/Idle/Fireman_Idle_Anim.Fireman_Idle_Anim"))))

(event Game|Damage|EventAnyDamage
  (params (Damage :type Float%20%28single-precision%29) (DamageType :type Damage%20Type%20Object%20Reference) (InstigatedBy :type Controller%20Object%20Reference) (DamageCauser :type Actor%20Object%20Reference))
  (CallFunction|GetDamagedbyEnemy Damage)
  (Sprite|SetSpriteColor (Variables|Default|GetFireman_Anim) "(R=1.000000,G=0.000000,B=0.000000,A=1.000000)")
  (Utilities|Time|SetTimerbyEvent (delegate Custom|HitMat) 0.2)
  (if (!= DamageCauser "BP_Fire")
    (Game|Damage|ApplyDamage 0 (Variables|Default|GetDamage) 0 self))
  (if (<= (Variables|Default|GetHealth) 0.0)
    (CallFunction|DefenseDeath)
    (Actor|DestroyActor)))

(event Collision|EventActorEndOverlap
  (params (OtherActor :type Actor%20Object%20Reference)))

(fn ConstructionScript)

(fn GetDamagedbyEnemy
  (params (EnemyDamage :type Float%20%28double-precision%29))
  (Variables|Default|SetHealth (- (Variables|Default|GetHealth) EnemyDamage))
  (return))

(fn DefenseDeath
  (Utilities|Array|RemoveItem (Variables|/Game/Blueprints/LvlComponents/BP_Detector.BP_Detector_C|GetDefendersLine (Variables|Default|GetDetectorRef)) self)
  (return))