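; BP_Detector is a defense-game trigger actor that tracks enemies entering its area and the defenders assigned to it.
; On overlap, it registers Basic-tagged enemies in EnemiesDetected, gives them a back-reference and calls the GameManager's UpdateDefenses.
; AddDefense records each defender, passes Archers or Guards the enemy list and detector reference, and deducts their cost from GameManager money.
; End overlap does nothing, so this Blueprint never removes enemies from its list.
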(event EventBeginPlay
  (bind _returnvalue (Actor|GetActorOfClass "/Game/Blueprints/GameManager.GameManager_C"))
  (Variables|Default|SetGameManRef _returnvalue))

(event Collision|EventActorEndOverlap
  (params (OtherActor :type Actor%20Object%20Reference)))

(event EventTick
  (params (DeltaSeconds :type Float%20%28single-precision%29)))

(event Collision|EventActorBeginOverlap
  (params (OtherActor :type Actor%20Object%20Reference))
  (if (Actor|ActorHasTag OtherActor "Enemy")
    (bind _array_element (Utilities|Array|ForEachLoopwithBreak (Variables|/Script/Engine.Actor|GetTags OtherActor) :!label _label)
      (:LoopBody
        (switch name _array_element
          (:Basic
            (bind _asbp_basic_enemy (Utilities|Casting|CastToBP_BasicEnemy OtherActor))
            (Variables|/Game/Blueprints/Enemies/BP_BasicEnemy.BP_BasicEnemy_C|SetDetectorRef _asbp_basic_enemy self)
            (Utilities|Array|Add (Variables|Default|GetEnemiesDetected) _asbp_basic_enemy)
            (Default|UpdateDefenses (Variables|Default|GetGameManRef) self)
            (goto _label Break)))))))

(fn ConstructionScript)

(fn AddDefense
  (params (DefenseToAdd :type Actor%20Object%20Reference) (SelectedDefense :type Integer))
  (bind _self self)
  (bind _enemiesdetected (Variables|Default|GetEnemiesDetected))
  (bind _gamemanref (Variables|Default|GetGameManRef))
  (Utilities|Array|Add (Variables|Default|GetDefendersLine) DefenseToAdd)
  (switch int SelectedDefense
    (:0
      (bind _asbp_archers (Utilities|Casting|CastToBP_Archers DefenseToAdd))
      (Variables|/Game/Blueprints/Defenses/BP_Archers.BP_Archers_C|SetEnemyList _asbp_archers _enemiesdetected)
      (Variables|/Game/Blueprints/Defenses/BP_Archers.BP_Archers_C|SetDetectorRef _asbp_archers _self)
      (Variables|/Game/Blueprints/GameManager.GameManager_C|SetMoney _gamemanref (- (Variables|/Game/Blueprints/GameManager.GameManager_C|GetMoney _gamemanref) (Variables|/Game/Blueprints/Defenses/BP_Archers.BP_Archers_C|GetCost _asbp_archers))))
    (:1
      (bind _asbp_guard (Utilities|Casting|CastToBP_Guard DefenseToAdd))
      (Variables|/Game/Blueprints/Defenses/BP_Guard.BP_Guard_C|SetEnemyList _asbp_guard _enemiesdetected)
      (Variables|/Game/Blueprints/Defenses/BP_Guard.BP_Guard_C|SetDetectorRef _asbp_guard _self)
      (Variables|/Game/Blueprints/GameManager.GameManager_C|SetMoney _gamemanref (- (Variables|/Game/Blueprints/GameManager.GameManager_C|GetMoney _gamemanref) (Variables|/Game/Blueprints/Defenses/BP_Guard.BP_Guard_C|GetCost _asbp_guard)))))
  (return))