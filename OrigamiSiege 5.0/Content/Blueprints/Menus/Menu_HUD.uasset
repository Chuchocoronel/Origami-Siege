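; Menu HUD actor that owns the main menu and level selection widgets and switches between them.
; On BeginPlay it creates both widgets, hands each a reference to itself, and adds only the main menu to the viewport.
; ReturntoMenu and GotoLevelSelection clear all widgets and re-add the cached one, so the menus navigate through the HUD without being recreated.
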(event EventBeginPlay
  (bind _self self)
  (Utilities|FlowControl|Sequence
    (:then_0
      (bind _returnvalue (UserInterface|CreateWidget "/Game/Blueprints/Menus/Main_Menu.Main_Menu_C"))
      (bind _output_get (Variables|Default|SetMainMenuRef _returnvalue))
      (Variables|/Game/Blueprints/Menus/Main_Menu.Main_Menu_C|SetMenuHUDRef _output_get _self)
      (UserInterface|Viewport|AddtoViewport _output_get 0))
    (:then_1
      (bind _returnvalue_2 (UserInterface|CreateWidget "/Game/Blueprints/Menus/LevelSelection_Menu.LevelSelection_Menu_C"))
      (bind _output_get_2 (Variables|Default|SetLevelSelectionRef _returnvalue_2))
      (Variables|/Game/Blueprints/Menus/LevelSelection_Menu.LevelSelection_Menu_C|SetMenuHUDRef _output_get_2 _self))))

(event Collision|EventActorBeginOverlap
  (params (OtherActor :type Actor%20Object%20Reference)))

(event EventTick
  (params (DeltaSeconds :type Float%20%28single-precision%29)))

(event EventReturntoMenu
  (Viewport|RemoveAllWidgets)
  (UserInterface|Viewport|AddtoViewport (Variables|Default|GetMainMenuRef) 0))

(event EventGotoLevelSelection
  (Viewport|RemoveAllWidgets)
  (UserInterface|Viewport|AddtoViewport (Variables|Default|GetLevelSelectionRef) 0))

(fn ConstructionScript)