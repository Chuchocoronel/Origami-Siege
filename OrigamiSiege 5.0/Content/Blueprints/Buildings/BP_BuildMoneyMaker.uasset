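; BP_BuildMoneyMaker is a building that periodically generates money for the player.
; A looping timer started on BeginPlay adds MoneyGeneration to the game manager's Money, refreshes the money notification and plays a sound at the building.
; A left click on the building resets the village UI message through the game manager.
; SubstractMoney&Check deducts a named defense's cost from the TypeDefensesData table and refreshes the notification, without checking affordability itself.
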(event Custom|GenerateMoney
  (bind _gamemanref (Variables|Default|GetGameManRef))
  ;[1 1 1] Generate money and update buttons
  (Variables|/Game/Blueprints/GameManager.GameManager_C|SetMoney _gamemanref (+ (Variables|/Game/Blueprints/GameManager.GameManager_C|GetMoney _gamemanref) (Variables|Default|GetMoneyGeneration)))
  (Class|WPBP|CheckNotificationMoney(Message) (Variables|Default|GetGameManRef))
  (Audio|PlaySoundatLocation "/Game/Music/Item_Sell_Purchase_05.Item_Sell_Purchase_05" (Transformation|GetActorLocation) "0, 0, 0" 1.0 1.0 0.0 "/Game/Music/Attenuation.Attenuation" 0 0 0))

(event EventBeginPlay
  ;[1 1 1] Generate money and update buttons
  (Utilities|Time|SetTimerbyEvent (delegate Custom|GenerateMoney) 1e+01 true))

(event Collision|EventActorBeginOverlap
  (params (OtherActor :type Actor%20Object%20Reference)))

(event EventTick
  (params (DeltaSeconds :type Float%20%28single-precision%29)))

(event MouseInput|EventActorOnClicked
  (params (ButtonPressed :type Key%20Structure :default "None"))
  (if (== ButtonPressed "LeftMouseButton")
    (Class|WPBP|ResetVillageUI(Message) (Variables|Default|GetGameManRef))))

(fn ConstructionScript)

(fn SubstractMoney&Check
  (params (Name%20Defense :type Name))
  (bind _gamemanref (Variables|Default|GetGameManRef))
  (bind _returnvalue (Utilities|GetDataTableRow "/Game/Blueprints/Defenses/TypeDefensesData.TypeDefensesData" Name%20Defense)
    (:then
      (Variables|/Game/Blueprints/GameManager.GameManager_C|SetMoney _gamemanref (- (Variables|/Game/Blueprints/GameManager.GameManager_C|GetMoney _gamemanref) (.cost _returnvalue)))
      (Class|WPBP|CheckNotificationMoney(Message) _gamemanref))))