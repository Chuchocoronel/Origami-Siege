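; Archery building that opens its recruitment UI through the game manager on left click and trains archers from a queue capped at six.
; Queuing an archer deducts its data-table cost immediately, then triggers a money notification check.
; A timer using the table's recruit time completes the front entry via the game manager and chains to the next.
; Each new order also re-sets that timer.
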(event Custom|RecuitEvent
  (bind _recuitqueue (Variables|Default|GetRecuitQueue))
  ;[1 1 1] Recuitment queue function
  (if (not (Utilities|Array|IsEmpty _recuitqueue))
    (bind _returnvalue (Utilities|GetDataTableRow "/Game/Blueprints/Defenses/TypeDefensesData.TypeDefensesData" (Utilities|Array|Get(acopy) _recuitqueue))
      (:then
        (Utilities|Time|SetTimerbyEvent (delegate Custom|Recuit) (.recuittime _returnvalue))))))

(event Custom|Recuit
  (bind _recuitqueue (Variables|Default|GetRecuitQueue))
  (bind _output (Utilities|Array|Get(acopy) _recuitqueue))
  ;[1 1 1] Recuitment queue function
  (switch name _output
    (:Archer
      (Default|RecuitArcher (Variables|Default|GetGameManRef))
      (Utilities|Array|RemoveIndex (Variables|Default|GetRecuitQueue))
      (if (not (Utilities|Array|IsEmpty _recuitqueue))
        (bind _returnvalue (Utilities|GetDataTableRow "/Game/Blueprints/Defenses/TypeDefensesData.TypeDefensesData" _output)
          (:then
            (Utilities|Time|SetTimerbyEvent (delegate Custom|Recuit) (.recuittime _returnvalue))))))))

(event EventBeginPlay)

(event Collision|EventActorBeginOverlap
  (params (OtherActor :type Actor%20Object%20Reference)))

(event EventTick
  (params (DeltaSeconds :type Float%20%28single-precision%29)))

(event EventRecuitArcher
  (bind _recuitqueue (Variables|Default|GetRecuitQueue))
  ;[1 1 1] Recuit archer and add to recuitment queue
  (if (< (Utilities|Array|Length _recuitqueue) 6)
    (Utilities|Array|Add _recuitqueue "Archer")
    (CallFunction|RecuitEvent)
    (CallFunction|SubstractMoney&Check "Archer")
    (else
      (Default|QueueFull (Variables|Default|GetGameManRef)))))

(event MouseInput|EventActorOnClicked
  (params (ButtonPressed :type Key%20Structure :default "None"))
  ;[1 1 1] Change UI to archery
  (if (== ButtonPressed "LeftMouseButton")
    (Class|UIInteractions|ArcheryUI(Message) (Variables|Default|GetGameManRef) self)))

(fn ConstructionScript)

(fn SubstractMoney&Check
  (params (Name%20Defense :type Name))
  (bind _gamemanref (Variables|Default|GetGameManRef))
  (bind _returnvalue (Utilities|GetDataTableRow "/Game/Blueprints/Defenses/TypeDefensesData.TypeDefensesData" Name%20Defense)
    (:then
      (Variables|/Game/Blueprints/GameManager.GameManager_C|SetMoney _gamemanref (- (Variables|/Game/Blueprints/GameManager.GameManager_C|GetMoney _gamemanref) (.cost _returnvalue)))
      (Class|WPBP|CheckNotificationMoney(Message) _gamemanref))))