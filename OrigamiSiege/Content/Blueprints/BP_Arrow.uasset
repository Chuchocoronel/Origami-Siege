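; BP_Arrow is a projectile actor that damages enemies on contact.
; Each tick it moves along the constant world right vector at Speed, scaled by delta time and without sweeping.
; On overlap with an "Enemy"-tagged BP_BasicEnemy, it subtracts Damage from Health, calls DestroyedEnemy if health runs out, then destroys itself.
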(event EventBeginPlay)

(event Collision|EventActorBeginOverlap
  (params (OtherActor :type Actor%20Object%20Reference))
  (if (!= (Utilities|Array|FindItem (Variables|/Script/Engine.Actor|GetTags OtherActor) "Enemy") -1)
    (bind _asbp_basic_enemy (Utilities|Casting|CastToBP_BasicEnemy OtherActor))
    (bind _output_get (Variables|/Game/Blueprints/BP_BasicEnemy.BP_BasicEnemy_C|SetHealth _asbp_basic_enemy (- (Variables|/Game/Blueprints/BP_BasicEnemy.BP_BasicEnemy_C|GetHealth _asbp_basic_enemy) (Variables|Default|GetDamage))))
    (if (<= _output_get 0.0)
      (Default|DestroyedEnemy _asbp_basic_enemy))
    (Actor|DestroyActor)))

(event EventTick
  (params (DeltaSeconds :type Float%20%28single-precision%29))
  (Transformation|AddActorWorldOffset (* (Class|KismetMathLibrary|VectorRight) (* DeltaSeconds (Variables|Default|GetSpeed)))))

(fn ConstructionScript)