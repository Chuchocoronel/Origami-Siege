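; BP_BasicEnemy is an enemy actor that moves every tick along its Direction at its Speed, without sweeping for collision.
; DestroyedEnemy loops over BP_Archers actors tagged Defense, removes an entry from each EnemyList and clears the AttackEnemy timer when a list empties.
; DestroyActor is called inside that loop, so it depends on at least one tagged archer being found.
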(event EventBeginPlay)

(event Collision|EventActorBeginOverlap
  (params (OtherActor :type Actor%20Object%20Reference)))

(event EventTick
  (params (DeltaSeconds :type Float%20%28single-precision%29))
  (Transformation|AddActorWorldOffset (* (Variables|Default|GetDirection) (* DeltaSeconds (Variables|Default|GetSpeed)))))

(fn ConstructionScript)

(fn DestroyedEnemy
  (bind _outactors (Actor|GetAllActorsOfClasswithTag "/Game/Blueprints/BP_Archers.BP_Archers_C" "Defense"))
  (for _array_element _outactors
    (Utilities|Array|RemoveItem (Variables|/Game/Blueprints/BP_Archers.BP_Archers_C|GetEnemyList _array_element) 0)
    (if (== (Utilities|Array|Length (Variables|/Game/Blueprints/BP_Archers.BP_Archers_C|GetEnemyList _array_element)) 0)
      (Utilities|Time|ClearTimerbyFunctionName _array_element "AttackEnemy"))
    (Actor|DestroyActor)))